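; Pinball bumper that knocks the ball away, awards points and plays a knock sound when a Ball-tagged component overlaps its sphere.
; It builds a velocity from the normalized bumper-to-ball direction with Z zeroed, scaled by ball speed and Force.
; It resets the ball's linear and angular velocities, applies that velocity as a mass-independent impulse, then reports Score to PinballGamemode.
; Debug prints of the locations and offset remain.
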(event OnComponentBeginOverlap(Sphere)
  (params (OverlappedComponent :type Primitive%20Component%20Object%20Reference) (OtherActor :type Actor%20Object%20Reference) (OtherComp :type Primitive%20Component%20Object%20Reference) (OtherBodyIndex :type Integer) (bFromSweep :type Boolean) (SweepResult :type Hit%20Result%20Structure%20%28by%20ref%29))
  (bind _defaultsceneroot (Variables|Default|GetDefaultSceneRoot))
  (bind _returnvalue (Transformation|GetWorldLocation _defaultsceneroot))
  ;[1 1 1] Bounce ball on collision
  (if (Components|ComponentHasTag OtherComp "Ball")
    (bind _asball (Utilities|Casting|CastToBall OtherActor))
    (Variables|Default|SetNewVelocity (* (* (* (Math|Vector|Normalize (- (Transformation|GetWorldLocation (Variables|/Game/Blueprints/Ball.Ball_C|GetSphere _asball)) _returnvalue)) "1.000000,1.000000,0.000000") (Math|Vector|VectorLength (Transformation|GetComponentVelocity (Variables|/Game/Blueprints/Ball.Ball_C|GetSphere _asball)))) (Variables|Default|GetForce)))
    ;;[1 1 1] Just for testing
    (Development|PrintString (Utilities|String|Append "Ball location: " (Utilities|String|ToString(Vector) (Transformation|GetWorldLocation (Variables|/Game/Blueprints/Ball.Ball_C|GetSphere _asball)))))
    (Development|PrintString (Utilities|String|Append "Bouncer Location:  " (Utilities|String|ToString(Vector) _returnvalue)))
    (Development|PrintString (Utilities|String|Append "Resultant Vector: " (Utilities|String|ToString(Vector) (- (Transformation|GetWorldLocation (Variables|/Game/Blueprints/Ball.Ball_C|GetSphere _asball)) _returnvalue))))
    (Physics|SetPhysicsLinearVelocity (Variables|/Game/Blueprints/Ball.Ball_C|GetSphere _asball) "0.000000,0.000000,1.000000" false "None")
    (Class|PrimitiveComponent|SetPhysicsAngularVelocityinDegrees (Variables|/Game/Blueprints/Ball.Ball_C|GetSphere _asball) "0, 0, 0" false "None")
    (Physics|AddImpulse (Variables|/Game/Blueprints/Ball.Ball_C|GetSphere _asball) (Variables|Default|GetNewVelocity) "None" true)
    ;[1 1 1] Add score
    (bind _aspinball_gamemode (Utilities|Casting|CastToPinballGamemode (Game|GetGameMode)))
    (Default|Scored _aspinball_gamemode (Variables|Default|GetScore))
    (Audio|Components|Audio|Play (Variables|Default|GetKnockCue) 0.0)))

(event EventBeginPlay)

(event Collision|EventActorBeginOverlap
  (params (OtherActor :type Actor%20Object%20Reference)))

(event EventTick
  (params (DeltaSeconds :type Float%20%28single-precision%29)))

(fn ConstructionScript)