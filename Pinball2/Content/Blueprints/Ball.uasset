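; Pinball ball actor that rolls under artificial gravity and reports when it is lost.
; Each Tick applies an acceleration along +Y to the Sphere and scales the RollingBall audio volume by the clamped, normalised speed.
; Overlapping a component tagged DeathPlane calls LostBall, which notifies PinballGamemode and then destroys the actor.
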(event OnComponentBeginOverlap(Sphere)
  (params (OverlappedComponent :type Primitive%20Component%20Object%20Reference) (OtherActor :type Actor%20Object%20Reference) (OtherComp :type Primitive%20Component%20Object%20Reference) (OtherBodyIndex :type Integer) (bFromSweep :type Boolean) (SweepResult :type Hit%20Result%20Structure%20%28by%20ref%29))
  (if (Components|ComponentHasTag OtherComp "DeathPlane")
    (CallFunction|LostBall)))

(event EventBeginPlay)

(event Collision|EventActorBeginOverlap
  (params (OtherActor :type Actor%20Object%20Reference)))

(event EventTick
  (params (DeltaSeconds :type Float%20%28single-precision%29))
  ;[1 1 1] Artificial gravity
  (Physics|AddForce (Variables|Default|GetSphere) "0.000000,600.000000,0.000000" "None" true)
  (Audio|Components|Audio|AdjustVolume (Variables|Default|GetRollingBall) 0.0 (/ (Math|Float|Clamp(Float) (Math|Vector|VectorLength (Transformation|GetComponentVelocity (Variables|Default|GetSphere))) 0.0 1.2e+03) 1.2e+03) "Linear" :!class /Script/Engine.AudioComponent))

(fn ConstructionScript)

(fn LostBall
  (bind _aspinball_gamemode (Utilities|Casting|CastToPinballGamemode (Game|GetGameMode)))
  (Default|BallLost _aspinball_gamemode)
  (Actor|DestroyActor))