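; Pinball paddle Blueprint that drives the left and right flippers from Enhanced Input and asks PinballGamemode to fire the ball.
; BeginPlay adds the IMC_Inputs mapping context to the player controller.
; AsyncPhysicsTick polls paddle inputs, playing or reversing timelines that yaw each hinge across a mirrored 40-degree arc.
; The right paddle check is nested in the left timeline's Update, so it runs only while that timeline updates.
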(event Input|EnhancedActionEvents|EnhancedInputActionIA_ShootBall
  (params (ActionValue :type Boolean) (ElapsedSeconds :type Float%20%28double-precision%29) (TriggeredSeconds :type Float%20%28double-precision%29) (InputAction :type Input%20Action%20Object%20Reference :default "/Game/INput/IA_ShootBall.IA_ShootBall"))
  (bind _aspinball_gamemode (Utilities|Casting|CastToPinballGamemode (Game|GetGameMode)))
  (Default|FireBall _aspinball_gamemode))

(event EventBeginPlay
  (bind _asplayer_controller (Utilities|Casting|CastToPlayerController (Pawn|GetController)))
  (Input|AddMappingContext (PlayerController|LocalPlayerSubsystems|GetEnhancedInputLocalPlayerSubsystem _asplayer_controller) "/Game/INput/IMC_Inputs.IMC_Inputs" 0 "(bIgnoreAllPressedKeysUntilRelease=True,bForceImmediately=False,bNotifyUserSettings=False)"))

(event Collision|EventActorBeginOverlap
  (params (OtherActor :type Actor%20Object%20Reference)))

(event EventTick
  (params (DeltaSeconds :type Float%20%28single-precision%29)))

(event EventAsyncPhysicsTick
  (params (DeltaSeconds :type Float%20%28single-precision%29) (SimSeconds :type Float%20%28single-precision%29))
  ;[1 1 1] Set left paddle to rotate
  (if (Input|EnhancedActionValues|GetIA_LeftPaddle)
    (bind _leftpaddle (Timeline|LeftpaddleTimeline Play)
      (:Update
        (CallFunction|SetLeftPaddleRotation _leftpaddle)
        ;[1 1 1] Set Right Paddle Rotation
        (if (Input|EnhancedActionValues|GetIA_RightPaddle)
          (bind _paddlerotation (Timeline|RightPaddleTimeline Play)
            (:Update
              (CallFunction|SetRightPaddleRotation _paddlerotation)))
          (else
            (Timeline|RightPaddleTimeline Reverse)))))
    (else
      (Timeline|LeftpaddleTimeline Reverse))))

(fn ConstructionScript)

(fn SetLeftPaddleRotation
  (params (Rotation :type Float%20%28double-precision%29))
  (Transformation|SetRelativeRotation (Variables|Default|GetLeftHinge) (Math|Rotator|MakeRotator 0.0 0.0 (* (- (* Rotation 4e+01) 2e+01) -1.0)) false false))

(fn SetRightPaddleRotation
  (params (Rotation :type Float%20%28double-precision%29))
  (Transformation|SetRelativeRotation (Variables|Default|GetRightHinge) (Math|Rotator|MakeRotator 0.0 0.0 (- (* Rotation 4e+01) 2e+01)) false false))