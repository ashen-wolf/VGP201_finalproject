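; Pinball game mode that tracks balls and score and ends the game when no balls remain.
; BeginPlay finds the BallSpawn actor, shows the playing HUD and pre-creates the game-over widget.
; FireBall launches a ball by impulse when none is in play, while it and Scored write updated values straight to the HUD.
; BallLost calls Lose at zero balls, which pauses, shows the final score and switches to UI-only input.
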(event EventBeginPlay
  (bind _returnvalue (Actor|GetActorOfClass "/Game/Blueprints/BallSpawn.BallSpawn_C"))
  (Variables|Default|SetBallSpawn _returnvalue)
  (bind _returnvalue_2 (UserInterface|CreateWidget "/Game/UI/PlayingUI.PlayingUI_C"))
  (bind _output_get (Variables|Default|SetPlayingWidget _returnvalue_2))
  (UserInterface|Viewport|AddtoViewport _output_get 0)
  (bind _returnvalue_3 (UserInterface|CreateWidget "/Game/UI/GameOver.GameOver_C"))
  (Variables|Default|SetGameOverWidget _returnvalue_3))

(event EventTick
  (params (DeltaSeconds :type Float%20%28single-precision%29)))

(fn ConstructionScript)

(fn BallLost
  (Math|Integer|DecrementInt (Variables|Default|GetBallsInPlay)
    (:%20%20
      (if (< (+ (Variables|Default|GetBallsInPlay) (Variables|Default|GetReserveBalls)) 1)
        (CallFunction|Lose)))))

(fn FireBall
  (if (< (Variables|Default|GetBallsInPlay) 1)
    ;[1 1 1] Create and shoot new ball
    (bind _returnvalue (Game|SpawnActorfromClass "/Game/Blueprints/Ball.Ball_C" (Transformation|GetActorTransform (Variables|Default|GetBallSpawn)) "Undefined" "MultiplyWithRoot" 0 0))
    (Physics|AddImpulse (Variables|/Game/Blueprints/Ball.Ball_C|GetSphere _returnvalue) "0.000000,-3000.000000,0.000000" "None" true)
    ;[1 1 1] Update all ball numbers
    (Math|Integer|DecrementInt (Variables|Default|GetReserveBalls)
      (:%20%20
        (Math|Integer|IncrementInt (Variables|Default|GetBallsInPlay)
          (:%20%20
            (bind _asplaying_ui (Utilities|Casting|CastToPlayingUI (Variables|Default|GetPlayingWidget)))
            (Rendering|Components|TextRender|SetText (Variables|/Game/UI/PlayingUI.PlayingUI_C|GetBalls _asplaying_ui) (Utilities|Text|ToText(String) (Utilities|String|Append "Balls: " (Utilities|String|ToString(Integer) (Variables|Default|GetReserveBalls)))))))))))

(fn Scored
  (params (score :type Float%20%28double-precision%29))
  (bind _output_get (Variables|Default|SetScore (+ score (Variables|Default|GetScore))))
  (bind _asplaying_ui (Utilities|Casting|CastToPlayingUI (Variables|Default|GetPlayingWidget)))
  (Rendering|Components|TextRender|SetText (Variables|/Game/UI/PlayingUI.PlayingUI_C|GetScore _asplaying_ui) (Utilities|Text|ToText(String) (Utilities|String|Append "Score: " (Utilities|String|ToString(Integer) (Math|Float|Round _output_get))))))

(fn Lose
  (bind _returnvalue (Game|GetPlayerController 0))
  (bind _gameoverwidget (Variables|Default|GetGameOverWidget))
  ;[1 1 1] End Game
  (Game|SetGamePaused true)
  (UserInterface|Viewport|AddtoViewport _gameoverwidget 0)
  (bind _asgame_over (Utilities|Casting|CastToGameOver _gameoverwidget))
  ;[1 1 1] Set visible score
  (Rendering|Components|TextRender|SetText (Variables|/Game/UI/GameOver.GameOver_C|GetScore _asgame_over) (Utilities|Text|ToText(String) (Utilities|String|Append "Score: " (Utilities|String|ToString(Integer) (Math|Float|Round (Variables|Default|GetScore))))))
  ;[1 1 1] Remove  Playing Widget
  (Widget|RemovefromParent (Variables|Default|GetPlayingWidget))
  (Variables|/Script/Engine.PlayerController|SetbShowMouseCursor _returnvalue true)
  (Input|SetInputModeUIOnly _returnvalue _asgame_over "DoNotLock" false))